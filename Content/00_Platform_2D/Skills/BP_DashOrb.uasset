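; BP_DashOrb is a pickup that grants the dash skill to the third-person character.
; It spins on its yaw axis each tick, and its sphere overlap calls GetDashSkill on the character.
; It then moves to the world origin, plays two drink sounds two seconds apart and destroys itself.
; The starting Z is stored on BeginPlay but not used here.
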(event OnComponentBeginOverlap(Sphere)
  (params (OverlappedComponent :type Primitive%20Component%20Object%20Reference) (OtherActor :type Actor%20Object%20Reference) (OtherComp :type Primitive%20Component%20Object%20Reference) (OtherBodyIndex :type Integer) (bFromSweep :type Boolean) (SweepResult :type Hit%20Result%20Structure%20%28by%20ref%29))
  (bind _asbp_third_person_character (Utilities|Casting|CastToBP_ThirdPersonCharacter OtherActor))
  (Default|GetDashSkill _asbp_third_person_character)
  (Transformation|SetActorLocation "0, 0, 0" false false)
  (Audio|PlaySound2D "/Game/00_Platform_2D/Sounds/drink1.drink1" 1.0 1.0 0.0 0 0)
  (Utilities|FlowControl|Delay 2.0)
  (Audio|PlaySound2D "/Game/00_Platform_2D/Sounds/drink2.drink2" 1.0 1.0 0.0 0 0)
  (Actor|DestroyActor))

(event EventBeginPlay
  (Variables|Default|SetInitialZ (.Z (Math|Vector|BreakVector (Transformation|GetActorLocation)))))

(event Collision|EventActorBeginOverlap
  (params (OtherActor :type Actor%20Object%20Reference)))

(event EventTick
  (params (DeltaSeconds :type Float%20%28single-precision%29))
  (Transformation|AddActorLocalRotation (Math|Rotator|MakeRotator 0.0 0.0 (* DeltaSeconds (Variables|Default|GetRotationSpeed))) false false))

(fn ConstructionScript)